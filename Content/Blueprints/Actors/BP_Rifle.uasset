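; BP_Rifle is a rifle weapon actor that adjusts its base damage according to whether the player or an enemy owns it.
; On the first Tick, a DoOnce gate compares the owner to player pawn 0 and multiplies BaseDamage by the player or enemy damage multiplier.
; BeginPlay and the construction script are empty, and this graph contains no firing logic.
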(event EventBeginPlay)

(event Collision|EventActorBeginOverlap
  (params (OtherActor :type Actor%20Object%20Reference)))

(event EventTick
  (params (DeltaSeconds :type Float%20%28single-precision%29))
  (Utilities|FlowControl|DoOnce false
    (:Completed
      (if (== (Components|GetOwner) (Game|Player|GetPlayerPawn 0))
        (Variables|Default|SetBaseDamage (* (Variables|Default|GetBaseDamage) (Variables|Default|GetPlayerDamageMultiplier)))
        (else
          (Variables|Default|SetBaseDamage (* (Variables|Default|GetBaseDamage) (Variables|Default|GetEnemyDamageMultiplier))))))))

(fn ConstructionScript)